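; GA_Blink is a gameplay ability that blinks the avatar Character in its direction of movement.
; On activation it commits, then rotates the actor's forward vector around Z by the velocity angle from CalculateDirection, falling back to forward if that vector is zero.
; It passes this direction and BlinkDistance to BlinkCharacter, whose body is not in this graph, then ends the ability.
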(event Ability|EventActivateAbility
  (bind _returnvalue (Ability|GetAvatarActorfromActorInfo))
  (bind _returnvalue_2 (Transformation|GetActorForwardVector _returnvalue))
  (Ability|CommitAbility)
  (bind _ascharacter (Utilities|Casting|CastToCharacter (Ability|GetAvatarActorfromActorInfo)))
  (Class|TLSBlinkSpell|BlinkCharacter (Math|Vector|SelectVector _returnvalue_2 (Math|Vector|Normalize (Math|Vector|RotateVectorAroundAxis _returnvalue_2 (Class|KismetAnimationLibrary|CalculateDirection (Variables|/Script/Engine.MovementComponent|GetVelocity (Variables|/Script/Engine.Character|GetCharacterMovement _ascharacter)) (Transformation|GetActorRotation _ascharacter)) "0.000000,0.000000,1.000000")) (Math|Vector|VectorIsZero (Math|Vector|Normalize (Math|Vector|RotateVectorAroundAxis _returnvalue_2 (Class|KismetAnimationLibrary|CalculateDirection (Variables|/Script/Engine.MovementComponent|GetVelocity (Variables|/Script/Engine.Character|GetCharacterMovement _ascharacter)) (Transformation|GetActorRotation _ascharacter)) "0.000000,0.000000,1.000000")))) (Variables|Default|GetBlinkDistance))
  (Ability|EndAbility))